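; BP_GameHUD is the game HUD that creates the UI widgets and sets the input mode for menu and gameplay.
; On BeginPlay it caches BP_GameModeBase, then shows the main menu with a cursor in MenuLevel, or the game overlay with game-only input in other levels.
; Tick polls the game mode's IsGameOver and uses a resettable DoOnce to show the game-over widget once, switching to UI-only input.
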(event EventBeginPlay
  (bind _returnvalue (Game|Player|GetOwningPlayerController))
  (bind _returnvalue_2 (Game|Player|GetOwningPlayerController))
  (Utilities|FlowControl|Sequence
    (:then_0
      (bind _asbp_game_mode_base (Utilities|Casting|CastToBP_GameModeBase (Game|GetGameMode)))
      (Variables|Default|SetGameMode _asbp_game_mode_base))
    (:then_1
      (bind _returnvalue_3 (Game|GetCurrentLevelName true))
      (if (Utilities|Enum|Equal(Enum) _returnvalue_3 "MenuLevel")
        (bind _returnvalue_4 (UserInterface|CreateWidget "/Game/UI/WBP_MainMenu.WBP_MainMenu_C"))
        (UserInterface|Viewport|AddtoViewport _returnvalue_4 0)
        (Input|SetInputModeUIOnly _returnvalue_2 0 "DoNotLock" false)
        (Variables|/Script/Engine.PlayerController|SetbShowMouseCursor _returnvalue_2 true)
        (else
          (bind _returnvalue_5 (UserInterface|CreateWidget "/Game/UI/WBP_GameOverlay.WBP_GameOverlay_C"))
          (UserInterface|Viewport|AddtoViewport _returnvalue_5 0)
          (Input|SetInputModeGameOnly _returnvalue false)
          (Variables|/Script/Engine.PlayerController|SetbShowMouseCursor _returnvalue false))))))

(event EventTick
  (params (DeltaSeconds :type Float%20%28single-precision%29))
  (bind _returnvalue (Game|Player|GetOwningPlayerController))
  (bind _result (Default|IsGameOver (Variables|Default|GetGameMode)))
  (if _result
    (Utilities|FlowControl|DoOnce false :!label _label
      (:Completed
        (bind _returnvalue_2 (UserInterface|CreateWidget "/Game/UI/WBP_GameOver.WBP_GameOver_C"))
        (UserInterface|Viewport|AddtoViewport _returnvalue_2 0)
        (Input|SetInputModeUIOnly _returnvalue 0 "DoNotLock" false)
        (Variables|/Script/Engine.PlayerController|SetbShowMouseCursor _returnvalue true)))
    (else
      (goto _label Reset))))

(fn ConstructionScript)